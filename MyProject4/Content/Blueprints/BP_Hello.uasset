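; BP_Hello is an actor that tests line tracing and reports what lies in front of it.
; On BeginPlay and every Tick it runs a debug-drawn Visibility trace from its root along the forward vector, scaled by a Distance variable.
; It prints the hit actor's name if tagged "item", a greeting for other hits, or a message when nothing is hit.
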(event `self.ReceiveBeginPlay`
  (bind _defaultsceneroot (`self.DefaultSceneRoot`))
  (bind _returnvalue (`SceneComponent.K2_GetComponentLocation` _defaultsceneroot))
  (bind (_outhit _returnvalue_2) (`KismetSystemLibrary.LineTraceSingle` :`Start` _returnvalue :`End` (+ _returnvalue (* (`KismetMathLibrary.GetForwardVector` (`SceneComponent.K2_GetComponentRotation` _defaultsceneroot)) (`self.Distance`))) :`TraceChannel` "TraceTypeQuery1" :`DrawDebugType` "ForDuration" :!label _label))
  (if _returnvalue_2
    (bind (_bblockinghit _binitialoverlap _time _distance _location _impactpoint _normal _impactnormal _physmat _hitactor) (`GameplayStatics.BreakHitResult` _outhit))
    (if (`self.ActorHasTag` _hitactor "item")
      (`KismetSystemLibrary.PrintString` (`KismetSystemLibrary.GetObjectName` _hitactor))
      (else
        (`KismetSystemLibrary.PrintString` "Hello")))
    (else
      (`KismetSystemLibrary.PrintString` "hit nothing"))))

(event `self.ReceiveTick`
  (params (DeltaSeconds :type "Float (single-precision)"))
  (goto _label))

(fn `UserConstructionScript`)